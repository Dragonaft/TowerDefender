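; Tower-defense tower that targets AiMob enemies within range and fires projectiles at them, configured from TowerStruct.
; It takes the first mob entering its range sphere and clears that target when it leaves; without a target, Tick runs throttled sphere traces to pick the closest mob.
; Shoot spawns a TowerProjectile with target and damage, gated by a fire-rate delay.
; Rotation is an empty stub, and the data-table lookup is disconnected.
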(event `self.ReceiveBeginPlay`
  (`self.TowerInit`))

(event `TowerInit`
  (`StaticMeshComponent.SetStaticMesh` (`self.TowerMesh`) (`.Mesh_12_E669ECF5495AC1156EB829BC13EE991D` (break `/Game/Tower/TowerStruct` (`self.Tower Struct`))))
  (`SphereComponent.SetSphereRadius` (`self.Sphere`) (`.Range_8_671CE41D4FFC52FDD0FFCF8FD108955E` (break `/Game/Tower/TowerStruct` (`self.Tower Struct`))) true))

(event `self.Sphere.OnComponentBeginOverlap`
  (params (OverlappedComponent :type "PrimitiveComponent Object Reference") (OtherActor :type "Actor Object Reference") (OtherComp :type "PrimitiveComponent Object Reference") (OtherBodyIndex :type Integer) (bFromSweep :type Boolean) (SweepResult :type "HitResult Structure (by ref)"))
  (`/Engine/EditorBlueprintResources/StandardMacros.IsValid` (`self.Target`)
    (:`Is Not Valid`
      (bind _asai_mob (cast `/Game/AI/AiMob` OtherActor))
      (set `self.Target` _asai_mob))))

(event `self.Sphere.OnComponentEndOverlap`
  (params (OverlappedComponent :type "PrimitiveComponent Object Reference") (OtherActor :type "Actor Object Reference") (OtherComp :type "PrimitiveComponent Object Reference") (OtherBodyIndex :type Integer))
  (if (== (`self.Target`) OtherActor)
    (set `self.Target` null)))

(event `Shoot`
  (bind (_name _damage _range _firerate) (break `/Game/Tower/TowerStruct` (`self.Tower Struct`)))
  (set `self.Reload` true)
  (`|SpawnActorFromClass` "/Game/Tower/TowerProjectile.TowerProjectile_C" (`self.GetTransform`) "AlwaysSpawn" "OverrideRootScale" null (`self.Target`) _damage null)
  (`KismetSystemLibrary.Delay` _firerate)
  (set `self.Reload` false))

(event `Rotation`)

(event `self.ReceiveTick`
  (params (DeltaSeconds :type "Float (single-precision)"))
  (`/Engine/EditorBlueprintResources/StandardMacros.IsValid` (`self.Target`)
    (:`Is Valid`
      (if (not (`self.Reload`))
        (`self.Shoot`)
        (`self.Rotation`)))
    (:`Is Not Valid`
      (if (not (`self.Check`))
        (`self.NewTarget`)))))

(event `NewTarget`
  (bind _returnvalue (`self.K2_GetActorLocation`))
  (set `self.Check` true)
  (bind (_outhits _returnvalue_2) (`KismetSystemLibrary.SphereTraceMultiForObjects` _returnvalue (- _returnvalue (0.0 0.0 1.0)) (`.Range_8_671CE41D4FFC52FDD0FFCF8FD108955E` (break `/Game/Tower/TowerStruct` (`self.Tower Struct`))) (`|MakeArray` "ObjectTypeQuery3" :!type "EObjectTypeQuery Enum")))
  (if _returnvalue_2
    (bind _target (`self.CloseTarget` _outhits))
    (`/Engine/EditorBlueprintResources/StandardMacros.IsValid` _target
      (:`Is Valid`
        (set `self.Target` _target))
      (:`Is Not Valid`
        _)))
  (`KismetSystemLibrary.Delay` 0.2)
  (set `self.Check` false))

(fn `CloseTarget`
  (params (HitResult :type "Array of HitResult Structure"))
  (returns (Target :type "/Game/AI/AiMob Object Reference"))
  (locals (TTarget :type "/Game/AI/AiMob Object Reference") (TDisatance :type "Float (double-precision)" :default 0.0))
  (for _array_element HitResult
    (bind (_bblockinghit _binitialoverlap _time _distance _location _impactpoint _normal _impactnormal _physmat _hitactor) (`GameplayStatics.BreakHitResult` _array_element))
    (bind _asai_mob (cast `/Game/AI/AiMob` _hitactor))
    (`/Engine/EditorBlueprintResources/StandardMacros.IsValid` (`local.TTarget`)
      (:`Is Valid`
        (bind _returnvalue (`KismetMathLibrary.VSize` (- (`self.K2_GetActorLocation`) (`self.K2_GetActorLocation` _hitactor))))
        (if (< _returnvalue (`local.TDisatance`))
          (set `local.TTarget` _asai_mob)
          (set `local.TDisatance` _returnvalue)))
      (:`Is Not Valid`
        (set `local.TTarget` _asai_mob)
        (set `local.TDisatance` _returnvalue))))
  (return (`local.TTarget`)))

(fn `UserConstructionScript`)